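; TheEnd is the end-of-level actor for the 2D shark scroller, scrolling toward negative X at a constant speed every tick.
; Its WinCollider calls WinGame on the shark controller, while Riser nudges the shark upward and JumpCollider launches it into the air on overlap.
; An Eraser volume destroys any overlapping actor tagged Culled.
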(event `self.ReceiveTick`
  (params (DeltaSeconds :type "Float (single-precision)"))
  ;[1 1 1] Movement
  (`self.K2_AddActorWorldOffset` (`KismetMathLibrary.MakeVector` (* DeltaSeconds 1000.0 -1.0))))

(event `self.WinCollider.OnComponentBeginOverlap`
  (params (OverlappedComponent :type "PrimitiveComponent Object Reference") (OtherActor :type "Actor Object Reference") (OtherComp :type "PrimitiveComponent Object Reference") (OtherBodyIndex :type Integer) (bFromSweep :type Boolean) (SweepResult :type "HitResult Structure (by ref)"))
  (bind _as2dshark_controller (cast `/Game/2DSharkScroller/Blueprints/2DSharkController` OtherActor))
  (`/Game/2DSharkScroller/Blueprints/2DSharkController.Win Game` _as2dshark_controller))

(event `self.Riser.OnComponentBeginOverlap`
  (params (OverlappedComponent :type "PrimitiveComponent Object Reference") (OtherActor :type "Actor Object Reference") (OtherComp :type "PrimitiveComponent Object Reference") (OtherBodyIndex :type Integer) (bFromSweep :type Boolean) (SweepResult :type "HitResult Structure (by ref)"))
  (bind _as2dshark_controller (cast `/Game/2DSharkScroller/Blueprints/2DSharkController` OtherActor))
  (`SceneComponent.K2_AddLocalOffset` (`Actor.RootComponent` _as2dshark_controller) (0.0 0.0 10.0) false false))

(event `self.JumpCollider.OnComponentBeginOverlap`
  (params (OverlappedComponent :type "PrimitiveComponent Object Reference") (OtherActor :type "Actor Object Reference") (OtherComp :type "PrimitiveComponent Object Reference") (OtherBodyIndex :type Integer) (bFromSweep :type Boolean) (SweepResult :type "HitResult Structure (by ref)"))
  (bind _as2dshark_controller (cast `/Game/2DSharkScroller/Blueprints/2DSharkController` OtherActor))
  (`Character.LaunchCharacter` _as2dshark_controller (0.0 0.0 1200.0) false false))

(event `self.Eraser.OnComponentBeginOverlap`
  (params (OverlappedComponent :type "PrimitiveComponent Object Reference") (OtherActor :type "Actor Object Reference") (OtherComp :type "PrimitiveComponent Object Reference") (OtherBodyIndex :type Integer) (bFromSweep :type Boolean) (SweepResult :type "HitResult Structure (by ref)"))
  (if (`self.ActorHasTag` OtherActor "Culled")
    (`self.K2_DestroyActor` OtherActor)))

(fn `UserConstructionScript`)