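; BuoyBP is a hazard for the 2D shark scroller that damages the player shark on overlap and then destroys itself.
; Tick scrolls it steadily along negative X, scaled by delta time, while bobbing it up or down by a fixed per-frame Z step.
; A looping one-second timer started on BeginPlay flips the GoingUp flag to reverse the bob.
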(event `self.ReceiveActorBeginOverlap`
  (params (OtherActor :type "Actor Object Reference"))
  ;[1 1 1] Damage Player
  (bind _as2dshark_controller (cast `/Game/2DSharkScroller/Blueprints/2DSharkController` OtherActor))
  (`/Game/2DSharkScroller/Blueprints/2DSharkController.Take Damage` _as2dshark_controller)
  (`self.K2_DestroyActor`))

(event `self.ReceiveTick`
  (params (DeltaSeconds :type "Float (single-precision)"))
  (bind _returnvalue_x (`KismetMathLibrary.BreakVector` (`KismetMathLibrary.MakeVector` (* DeltaSeconds 400.0 -1.0))))
  ;[1 1 1] Movement
  (if (`self.GoingUp`)
    (`self.K2_AddActorWorldOffset` (`KismetMathLibrary.MakeVector` _returnvalue_x 0.0 0.5))
    (else
      (`self.K2_AddActorWorldOffset` (`KismetMathLibrary.MakeVector` _returnvalue_x 0.0 -0.5)))))

(event `self.ReceiveBeginPlay`
  ;[1 1 1] Movement
  (`KismetSystemLibrary.K2_SetTimerDelegate` (delegate `Toggle`) 1.0 true))

(event `Toggle`
  ;[1 1 1] Movement
  (if (`self.GoingUp`)
    (set `self.GoingUp` false)
    (else
      (set `self.GoingUp` true))))

(fn `UserConstructionScript`)